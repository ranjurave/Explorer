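; BP_Cannon is a turret actor that turns toward the player and fires projectiles when it has line of sight.
; Each Tick it traces on Visibility from its Sphere component to the player character, continuing only if the hit actor is a BP_Mutant.
; It then rotates on yaw only to face the player and spawns a BP_Projectile at the Sphere's transform, every qualifying frame with no cooldown.
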(event `self.ReceiveTick`
  (params (DeltaSeconds :type "Float (single-precision)"))
  (bind _outhit (`KismetSystemLibrary.LineTraceSingle` :`Start` (`SceneComponent.K2_GetComponentLocation` (`self.Sphere`)) :`End` (`self.K2_GetActorLocation` (`GameplayStatics.GetPlayerCharacter` 0)) :`TraceChannel` "TraceTypeQuery1" :`DrawDebugType` "ForOneFrame"))
  (cast `/Game/Blueprints/BP_Mutant` (`.HitActor` (`GameplayStatics.BreakHitResult` _outhit)))
  (`self.K2_SetActorRotation` (`KismetMathLibrary.MakeRotator` 0.0 0.0 (.yaw (`KismetMathLibrary.FindLookAtRotation` (`self.K2_GetActorLocation`) (`self.K2_GetActorLocation` (`GameplayStatics.GetPlayerCharacter` 0))))))
  (`|SpawnActorFromClass` "/Game/Blueprints/BP_Projectile.BP_Projectile_C" (`SceneComponent.K2_GetComponentToWorld` (`self.Sphere`)) "AlwaysSpawn" "MultiplyWithRoot" null null))

(fn `UserConstructionScript`)